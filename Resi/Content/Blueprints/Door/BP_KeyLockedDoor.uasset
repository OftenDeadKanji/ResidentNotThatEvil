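; BP_KeyLockedDoor is a door Blueprint that keeps its mesh animation in step with the door's state; no key or lock logic appears in its graphs.
; On BeginPlay it applies CurrentState to the animation, then binds to the start and finish events for opening and closing.
; Each path calls SetAnimationTransitionVariables, which writes all four CanEnter transition flags on ABP_Door, enabling only the matching one.
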(event Custom|OnDoorStartClosing_Event
  (CallFunction|SetAnimationTransitionVariables false true false false))

(event Custom|OnDoorFinishClosing_Event
  (CallFunction|SetAnimationTransitionVariables true false false false))

(event Custom|OnDoorStartOpening_Event
  (CallFunction|SetAnimationTransitionVariables false false false true))

(event Custom|OnDoorFinishOpening_Event
  (CallFunction|SetAnimationTransitionVariables false false true false))

(event EventBeginPlay
  (Utilities|FlowControl|Sequence
    (:then_0
      (switch Utilities|FlowControl|Switch|SwitchonEDoorState (Variables|Default|GetCurrentState)
        (:Closed
          (CallFunction|SetAnimationTransitionVariables true false false false))
        (:Closing
          (CallFunction|SetAnimationTransitionVariables false true false false))
        (:Open
          (CallFunction|SetAnimationTransitionVariables false false true false))
        (:Opening
          (CallFunction|SetAnimationTransitionVariables false false false true))))
    (:then_1
      (EventDispatchers|AssignOnDoorStartClosing (delegate Custom|OnDoorStartClosing_Event))
      (EventDispatchers|AssignOnDoorFinishClosing (delegate Custom|OnDoorFinishClosing_Event))
      (EventDispatchers|AssignOnDoorStartOpening (delegate Custom|OnDoorStartOpening_Event))
      (EventDispatchers|AssignOnDoorFinishOpening (delegate Custom|OnDoorFinishOpening_Event)))))

(fn ConstructionScript)

(fn SetAnimationTransitionVariables
  (params (CanEnterClosed :type Boolean) (CanEnterClosing :type Boolean) (CanEnterOpen :type Boolean) (CanEnterOpening :type Boolean))
  (bind _asabp_door (Utilities|Casting|CastToABP_Door (Components|SkeletalMesh|GetAnimInstance (Variables|Character|GetMesh))))
  (Variables|/Game/Meshes/Door/Animations/ABP_Door.ABP_Door_C|SetCanEnterClosed _asabp_door CanEnterClosed)
  (Variables|/Game/Meshes/Door/Animations/ABP_Door.ABP_Door_C|SetCanEnterClosing _asabp_door CanEnterClosing)
  (Variables|/Game/Meshes/Door/Animations/ABP_Door.ABP_Door_C|SetCanEnterOpen _asabp_door CanEnterOpen)
  (Variables|/Game/Meshes/Door/Animations/ABP_Door.ABP_Door_C|SetCanEnterOpening _asabp_door CanEnterOpening))